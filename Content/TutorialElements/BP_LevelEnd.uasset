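; BP_LevelEnd is a tutorial level exit that loads the next level when the player has a key.
; When an actor tagged Player overlaps the Box trigger, it sends a CheckHasKey message to that actor to query key possession.
; A positive result opens the level set in LevelName.
; Otherwise the TextRender, hidden at BeginPlay, appears briefly and hides again after a delay.
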(event OnComponentBeginOverlap(Box)
  (params (OverlappedComponent :type Primitive%20Component%20Object%20Reference) (OtherActor :type Actor%20Object%20Reference) (OtherComp :type Primitive%20Component%20Object%20Reference) (OtherBodyIndex :type Integer) (bFromSweep :type Boolean) (SweepResult :type Hit%20Result%20Structure%20%28by%20ref%29))
  (if (Actor|ActorHasTag OtherActor "Player")
    (bind _haskey (Class|BPIPlayer|CheckHasKey(Message) OtherActor))
    (if _haskey
      (Game|OpenLevel(byName) (Variables|Default|GetlevelName))
      (else
        (Rendering|SetVisibility (Variables|Default|GetTextRender) true false)
        (Utilities|FlowControl|Delay 3.0)
        (Rendering|SetVisibility (Variables|Default|GetTextRender) false false)))))

(event EventBeginPlay
  (Rendering|SetVisibility (Variables|Default|GetTextRender) false false))

(event Collision|EventActorBeginOverlap
  (params (OtherActor :type Actor%20Object%20Reference)))

(event EventTick
  (params (DeltaSeconds :type Float%20%28single-precision%29)))

(fn ConstructionScript)