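; Procedural level generator test actor that builds a row of mesh segments along the X axis on BeginPlay and caps it with a BP_LevelEnd.
; Each BP_SpawnedMesh gets a random mesh, re-rolled to avoid repeating the previous one.
; A coin flip picks horizontal or vertical BP_MovingPlatform travel of random distance, skipped for certain meshes.
; Some mesh types also have a 50/50 chance of a random pickup.
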(event EventBeginPlay
  (bind _returnvalue (Math|Random|RandomFloatinRange 2.8e+02 4e+02))
  (bind _returnvalue_2 (Transformation|GetActorTransform))
  (bind _pickups (Variables|Default|GetpickUps))
  (bind _returnvalue_3 (+ (.z (.location _returnvalue_2)) 285.0))
  (for _index (range 0 (- (Variables|Default|GetnumOfSpawned) 1))
    (bind _returnvalue_4 (Game|SpawnActorfromClass "/Game/Procedural/BP_SpawnedMesh.BP_SpawnedMesh_C" (Math|Transform|MakeTransform (Math|Vector|MakeVector (+ (.x (.location _returnvalue_2)) (Math|Conversions|ToFloat(Integer) (* _index 800))) (.y (.location _returnvalue_2)) (.z (.location _returnvalue_2))) "0, 0, 0" "1.000000,1.000000,1.000000") "Undefined" "MultiplyWithRoot" 0 0))
    ;[0 0.03245 1] Comparación con mesh spawneado anteriormente
    (bind _output_get (Variables|Default|SetcurrentMeshIndex (Math|Random|RandomIntegerinRange 0 (- (Utilities|Array|Length (Variables|Default|GetMeshes)) 1)) :!label _label))
    (if (== _output_get (Variables|Default|GetpreviousMeshIndex))
      (goto _label)
      (else
        (Components|StaticMesh|SetStaticMesh (Variables|/Game/Procedural/BP_SpawnedMesh.BP_SpawnedMesh_C|GetStaticMesh _returnvalue_4) (Utilities|Array|Get(acopy) (Variables|Default|GetMeshes) _output_get))
        (Variables|Default|SetpreviousMeshIndex _output_get)
        ;[0 0.01971 1] 50/50 plataforma vertical u horizontal
        (if (Math|Random|RandomBool)
          (if (== (Variables|Default|GetcurrentMeshIndex) 1)
            _
            (else
              (Game|SpawnActorfromClass "/Game/Procedural/BP_MovingPlatform.BP_MovingPlatform_C" (Math|Transform|MakeTransform (Math|Vector|MakeVector (+ (+ (.x (.location _returnvalue_2)) (Math|Conversions|ToFloat(Integer) (* _index 800))) 4e+02) (.y (.location _returnvalue_2)) _returnvalue_3) "0, 0, 0" "1.000000,1.000000,1.000000") "Undefined" "MultiplyWithRoot" 0 (Math|Vector|MakeVector _returnvalue 0.0 0.0) 0)))
          (elif (== (Variables|Default|GetcurrentMeshIndex) 2)
            _
            (else
              (Game|SpawnActorfromClass "/Game/Procedural/BP_MovingPlatform.BP_MovingPlatform_C" (Math|Transform|MakeTransform (Math|Vector|MakeVector (+ (+ (.x (.location _returnvalue_2)) (Math|Conversions|ToFloat(Integer) (* _index 800))) 4e+02) (.y (.location _returnvalue_2)) _returnvalue_3) "0, 0, 0" "1.000000,1.000000,1.000000") "Undefined" "MultiplyWithRoot" 0 (Math|Vector|MakeVector 0.0 0.0 _returnvalue) 0))))
        (if (or (== (Variables|Default|GetcurrentMeshIndex) 0) (== (Variables|Default|GetcurrentMeshIndex) 3))
          (if (Math|Random|RandomBool)
            (Game|SpawnActorfromClass (Utilities|Array|Get(acopy) _pickups (Math|Random|RandomIntegerinRange 0 (Utilities|Array|Length _pickups))) (Math|Transform|MakeTransform (Math|Vector|MakeVector (+ (+ (.x (.location _returnvalue_2)) (Math|Conversions|ToFloat(Integer) (* _index 800))) 4e+02) (.y (.location _returnvalue_2)) (+ (.z (.location _returnvalue_2)) 4e+02)) "0, 0, 0" "1.000000,1.000000,1.000000") "Undefined" "MultiplyWithRoot" 0 0))))))
  (Game|SpawnActorfromClass "/Game/TutorialElements/BP_LevelEnd.BP_LevelEnd_C" (Math|Transform|MakeTransform (Math|Vector|MakeVector (+ (+ (.x (.location _returnvalue_2)) (Math|Conversions|ToFloat(Integer) (* _index 800))) 4e+02) (.y (.location _returnvalue_2)) (+ (.z (.location _returnvalue_2)) 2e+02)) "0, 0, 0" "1.000000,1.000000,1.000000") "Undefined" "MultiplyWithRoot" 0 0))

(fn ConstructionScript)