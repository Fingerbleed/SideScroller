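; BP_BackgroundGenerator procedurally builds a background row of randomly chosen sprites when play begins.
; It spawns BP_SpawnedSprite actors along the X axis from its own location, spaced by Distance, with the count driven by NumOfRepetitions.
; Each spawn gets a configurable Z scale, a random sprite from the Sprites array, and its point light shown or hidden by UsesLight.
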(event EventBeginPlay
  (bind _returnvalue (Transformation|GetActorLocation))
  (bind _sprites (Variables|Default|Getsprites))
  (for _index (range 0 (Variables|Default|GetnumOfRepetitions))
    (bind _returnvalue_2 (Game|SpawnActorfromClass "/Game/Procedural/BP_SpawnedSprite.BP_SpawnedSprite_C" (Math|Transform|MakeTransform (Math|Vector|MakeVector (+ (.x _returnvalue) (Math|Conversions|ToFloat(Integer) (* _index (Variables|Default|Getdistance)))) (.y _returnvalue) (.z _returnvalue)) "0, 0, 0" (Math|Vector|MakeVector 1.0 1.0 (Variables|Default|GetSpawn%20Transform%20Scale%20Z))) "Undefined" "MultiplyWithRoot" 0 0))
    (Rendering|Components|Sprite|SetSprite (Variables|/Game/Procedural/BP_SpawnedSprite.BP_SpawnedSprite_C|GetPaperSprite _returnvalue_2) (Utilities|Array|Get(acopy) _sprites (Math|Random|RandomIntegerinRange 0 (- (Utilities|Array|Length _sprites) 1))))
    (Rendering|SetVisibility (Variables|/Game/Procedural/BP_SpawnedSprite.BP_SpawnedSprite_C|GetPointLight _returnvalue_2) (Variables|Default|GetusesLight) false)))

(event Collision|EventActorBeginOverlap
  (params (OtherActor :type Actor%20Object%20Reference)))

(event EventTick
  (params (DeltaSeconds :type Float%20%28single-precision%29)))

(fn ConstructionScript)