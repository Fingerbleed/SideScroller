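; BP_NPC1 is an enemy NPC that spots the player, attacks in melee and can drop pickups on death.
; Pawn sensing sets the "HasSeenPlayer?" blackboard key, and AttackPlayer1 damages a player hit by a short forward sphere trace.
; At zero health, chained random rolls choose a torch or armor polish; the laudanum roll can never pass.
; The actor is destroyed only when a pickup spawns.
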(event OnSeePawn(PawnSensing)
  (params (Pawn :type Pawn%20Object%20Reference))
  (Utilities|Casting|CastToBP_Player Pawn)
  (AI|Components|Blackboard|SetValueasBool (AI|GetBlackboard (AI|GetAIController self)) (Utilities|Name|MakeLiteralName "HasSeenPlayer?") true))

(event Custom|AttackPlayer1
  (bind _returnvalue (Transformation|GetActorLocation))
  (bind (_outhit _returnvalue_2) (Collision|SphereTraceForObjects _returnvalue (+ _returnvalue (* (Math|Vector|GetForwardVector (Transformation|GetActorRotation)) 2.5e+02)) 45.0 (Utilities|Array|MakeArray "ObjectTypeQuery3") false 0 "None"))
  (if _returnvalue_2
    (Utilities|Casting|CastToBP_Player (.HitActor (Collision|BreakHitResult _outhit)))
    (Game|Damage|ApplyDamage (.HitActor (Collision|BreakHitResult _outhit)) 1e+01 0 self)))

(event EventBeginPlay)

(event Collision|EventActorBeginOverlap
  (params (OtherActor :type Actor%20Object%20Reference)))

(event EventTick
  (params (DeltaSeconds :type Float%20%28single-precision%29)))

(event Game|Damage|EventAnyDamage
  (params (Damage :type Float%20%28single-precision%29) (DamageType :type Damage%20Type%20Object%20Reference) (InstigatedBy :type Controller%20Object%20Reference) (DamageCauser :type Actor%20Object%20Reference))
  (bind _returnvalue (Math|Random|RandomInteger 10))
  (bind _papersprite (Variables|Default|GetPaperSprite))
  (bind _returnvalue_2 (Transformation|GetWorldLocation _papersprite))
  (Variables|Default|SetHealth (- (Variables|Default|GetHealth) Damage))
  (if (<= (Variables|Default|GetHealth) 0.0)
    (Variables|Default|SetisDead? true)
    (if (> _returnvalue 9)
      (Game|SpawnActorfromClass "/Game/PickUps/LaudanumPickUp.LaudanumPickUp_C" (Math|Transform|MakeTransform _returnvalue_2 "0, 0, 0" "1.000000,1.000000,1.000000") "Undefined" "MultiplyWithRoot" 0 0)
      (Actor|DestroyActor :!label _label)
      (elif (> _returnvalue 8)
        (Game|SpawnActorfromClass "/Game/PickUps/TorchPickUp.TorchPickUp_C" (Math|Transform|MakeTransform _returnvalue_2 "0, 0, 0" "1.000000,1.000000,1.000000") "Undefined" "MultiplyWithRoot" 0 0)
        (goto _label)
        (elif (> _returnvalue 6)
          (Game|SpawnActorfromClass "/Game/PickUps/ArmorPolishPickUp.ArmorPolishPickUp_C" (Math|Transform|MakeTransform _returnvalue_2 "0, 0, 0" "1.000000,1.000000,1.000000") "Undefined" "MultiplyWithRoot" 0 0)
          (goto _label))))))

(fn ConstructionScript)