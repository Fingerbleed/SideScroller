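; Side-scrolling player character with walk, run, crouch, jump, sword attack and directional shield, plus key and torch hooks.
; Enhanced Input drives actions gated by state flags and delays, with sphere traces for hits and headroom.
; Frontal enemy hits are parried for a brief damage boost or blocked with knockback and random shield wear; others hurt, granting brief invulnerability.
; Health feeds an interface-driven HUD, and death reloads the level.
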(event Custom|Interface%20Setup
  ;[0 0 0] Interface Setup
  (bind _player_interface (Class|BPIGameInstance|GetPlayerInterface(Message) (Game|GetGameInstance)))
  (Utilities|IsValid _player_interface
    (:Is%20Valid
      (bind _output_get (Variables|Default|SetPlayerInterface _player_interface))
      (UserInterface|Viewport|AddtoViewport _output_get 0))))

(event Custom|Add%20Mapping
  (bind _returnvalue (Game|GetPlayerController 0))
  (bind _returnvalue_2 (PlayerController|LocalPlayerSubsystems|GetEnhancedInputLocalPlayerSubsystem _returnvalue))
  ;[0 0 0] Input Mapping
  (Utilities|IsValid _returnvalue_2
    (:Is%20Valid
      (Input|AddMappingContext _returnvalue_2 "/Game/Player/Blueprints/Input/IMC_Player.IMC_Player" 0 "(bIgnoreAllPressedKeysUntilRelease=True,bForceImmediately=False)"))))

(event Custom|Set%20Rotation
  (bind _sprite (Variables|Default|GetSprite))
  ;[0 0 0] Rotation
  (Math|Float|CompareFloat (.x (Variables|/Script/Engine.MovementComponent|GetVelocity (Variables|Character|GetCharacterMovement))) 0.0
    (:>
      (Transformation|SetRelativeRotation _sprite "0, 0, 0" false false))
    (:<
      (Transformation|SetRelativeRotation _sprite "0.000000,180.000000,0.000000" false false))))

(event Custom|Stop%20Crouching
  (bind _sprite (Variables|Default|GetSprite))
  (bind _returnvalue (Transformation|GetWorldLocation _sprite))
  ;[0 0 0] Movement
  (if (AI|Components|NavMovement|IsCrouching (Variables|Character|GetCharacterMovement))
    (bind (_outhit _returnvalue_2) (Collision|SphereTraceByChannel _returnvalue (+ _returnvalue "0.000000,0.000000,25.000000") 5e+01 "TraceTypeQuery1" false 0 "None"))
    (if _returnvalue_2
      (if (Actor|ActorHasTag (.hitactor _outhit) "Trigger")
        (Character|UnCrouch :!label _label)
        (Transformation|AddLocalOffset (Variables|Default|GetSprite) (Math|Vector|MakeVector 0.0 0.0 (* (Variables|Default|GetCrouchOffset) -1.0)) false false))
      (else
        (goto _label)))))

(event Custom|Get%20Hit
  (params (Damage :type Float%20%28double-precision%29))
  ;[0 0 0] Take Damage
  (CallFunction|TakeDamage Damage)
  (Audio|PlaySound2D "/Game/Sounds/Player/AAAAA.AAAAA" 1.0 1.0 0.0 0 0)
  (Character|LaunchCharacter "0.000000,0.000000,350.000000" false false)
  (Variables|Default|SetCanTakeDamage false)
  (Utilities|FlowControl|Delay (Variables|Default|GetInvencibilityTime))
  (Variables|Default|SetCanTakeDamage true))

(event Custom|UpdateMovementSound
  (bind _returnvalue (Transformation|GetVelocity))
  (bind _walkruncrouchspeed (Variables|Default|GetWalkRunCrouchSpeed))
  (bind _movementaudio (Variables|Default|GetMovementAudio))
  (bind _movementaudio_2 (Variables|Default|GetMovementAudio))
  (bind _movementaudio_3 (Variables|Default|GetMovementAudio))
  (bind _returnvalue_2 (Math|Float|Absolute(Float) (.x _returnvalue)))
  ;[0 0 0] Movement Audio
  (if (or (== _returnvalue_2 0.0) (!= (.z _returnvalue) 0.0))
    (Audio|Components|Audio|Stop _movementaudio_2)
    (else
      (if (Variables|Default|GetIsShielded)
        (if (== (Variables|/Script/Engine.AudioComponent|GetPitchMultiplier _movementaudio_3) 0.8) :!label _label
          _
          (else
            (Audio|Components|Audio|SetPitchMultiplier _movementaudio_2 0.8)))
        (elif (== _returnvalue_2 (.x _walkruncrouchspeed))
          (if (== (Variables|/Script/Engine.AudioComponent|GetPitchMultiplier _movementaudio_3) 1.5)
            _
            (else
              (Audio|Components|Audio|SetPitchMultiplier _movementaudio_2 1.5)))
          (elif (>= _returnvalue_2 (.y _walkruncrouchspeed))
            (if (== (Variables|/Script/Engine.AudioComponent|GetPitchMultiplier _movementaudio_3) 2.0)
              _
              (else
                (Audio|Components|Audio|SetPitchMultiplier _movementaudio_2 2.0)))
            (else
              (goto _label)))))
      (if (not (Audio|Components|Audio|IsPlaying _movementaudio))
        (Audio|Components|Audio|Play _movementaudio 0.0)))))

(event Custom|FallSound
  (bind _returnvalue (Transformation|GetVelocity))
  (if (Variables|Default|GetcanPlayFallSound)
    (if (== (.z _returnvalue) 0.0)
      (Variables|Default|SetcanPlayFallSound false)
      (Audio|PlaySound2D "/Game/Sounds/Player/Fall.Fall" 1.0 1.0 0.0 0 0))
    (elif (!= (.z _returnvalue) 0.0)
      (Variables|Default|SetcanPlayFallSound true))))

(event Input|EnhancedActionEvents|EnhancedInputActionIA_Run
  (params (ActionValue :type Float%20%28double-precision%29) (ElapsedSeconds :type Float%20%28double-precision%29) (TriggeredSeconds :type Float%20%28double-precision%29) (InputAction :type Input%20Action%20Object%20Reference :default "/Game/Player/Blueprints/Input/IA_Run.IA_Run"))
  (bind _charactermovement (Variables|Character|GetCharacterMovement))
  (bind _walkruncrouchspeed (Variables|Default|GetWalkRunCrouchSpeed))
  ;[0 0 0] Movement
  (:Triggered
    (if (not (Variables|Default|GetIsShielded))
      (Variables|/Script/Engine.CharacterMovementComponent|SetMaxWalkSpeed _charactermovement (.y _walkruncrouchspeed))))
  (:Completed
    (if (not (Variables|Default|GetIsShielded))
      (Variables|/Script/Engine.CharacterMovementComponent|SetMaxWalkSpeed _charactermovement (.x _walkruncrouchspeed)))))

(event Input|EnhancedActionEvents|EnhancedInputActionIA_Move
  (params (ActionValue :type Float%20%28double-precision%29) (ElapsedSeconds :type Float%20%28double-precision%29) (TriggeredSeconds :type Float%20%28double-precision%29) (InputAction :type Input%20Action%20Object%20Reference :default "/Game/Player/Blueprints/Input/IA_Move.IA_Move"))
  ;[0 0 0] Movement
  (:Triggered
    (if (not (Variables|Default|GetIsAttacking))
      (Pawn|Input|AddMovementInput "1.000000,0.000000,0.000000" ActionValue false)
      (Math|Float|CompareFloat ActionValue 0.0
        (:>
          (Variables|Default|SetlastDirection 1))
        (:<
          (Variables|Default|SetlastDirection -1))))))

(event Input|EnhancedActionEvents|EnhancedInputActionIA_Jump
  (params (ActionValue :type Float%20%28double-precision%29) (ElapsedSeconds :type Float%20%28double-precision%29) (TriggeredSeconds :type Float%20%28double-precision%29) (InputAction :type Input%20Action%20Object%20Reference :default "/Game/Player/Blueprints/Input/IA_Jump.IA_Jump"))
  ;[0 0 0] Movement
  (:Triggered
    (if (not (and (Variables|Default|GetIsShielded) (Variables|Default|GetIsAttacking)))
      (CallFunction|StopCrouching)
      (if (not (AI|Components|NavMovement|IsCrouching (Variables|Character|GetCharacterMovement)))
        (Character|Jump)
        ;[0 0 0] Shield
        (Variables|Default|SetIsShielded false)
        (Variables|Default|SetcanShield false)
        (Variables|/Script/Engine.CharacterMovementComponent|SetMaxWalkSpeed (Variables|Character|GetCharacterMovement) (.x (Variables|Default|GetWalkRunCrouchSpeed)))
        (Utilities|FlowControl|Delay 0.25)
        (Variables|Default|SetcanShield true))))
  (:Started
    (if (not (Variables|Default|GetIsShielded))
      (if (== (.z (Transformation|GetVelocity)) 0.0)
        (Audio|PlaySound2D "/Game/Sounds/Player/Jump.Jump" 1.0 1.0 0.0 0 0))))
  (:Completed
    (Character|StopJumping)))

(event Input|EnhancedActionEvents|EnhancedInputActionIA_Crouch
  (params (ActionValue :type Float%20%28double-precision%29) (ElapsedSeconds :type Float%20%28double-precision%29) (TriggeredSeconds :type Float%20%28double-precision%29) (InputAction :type Input%20Action%20Object%20Reference :default "/Game/Player/Blueprints/Input/IA_Crouch.IA_Crouch"))
  ;[0 0 0] Movement
  (:Started
    (Variables|Default|SetCrouchpress true)
    (if (not (AI|Components|NavMovement|IsCrouching (Variables|Character|GetCharacterMovement)))
      (if (not (Variables|Default|GetIsShielded))
        (if (== 0.0 (.z (Transformation|GetVelocity)))
          (Character|Crouch)
          (Transformation|AddLocalOffset (Variables|Default|GetSprite) (Math|Vector|MakeVector 0.0 0.0 (Variables|Default|GetCrouchOffset)) false false)))))
  (:Completed
    (Variables|Default|SetCrouchpress false)
    (CallFunction|StopCrouching)))

(event Input|EnhancedActionEvents|EnhancedInputActionIA_Attack
  (params (ActionValue :type Float%20%28double-precision%29) (ElapsedSeconds :type Float%20%28double-precision%29) (TriggeredSeconds :type Float%20%28double-precision%29) (InputAction :type Input%20Action%20Object%20Reference :default "/Game/Player/Blueprints/Input/IA_Attack.IA_Attack"))
  (bind _lastdirection (Variables|Default|GetlastDirection))
  (bind _sprite (Variables|Default|GetSprite))
  (bind _attackdamage (Variables|Default|GetAttackDamage))
  (bind _returnvalue (Transformation|GetWorldLocation _sprite))
  (bind _returnvalue_2 (* _lastdirection 50))
  (bind _returnvalue_3 (+ _returnvalue (Math|Vector|MakeVector _returnvalue_2 0.0 12.5)))
  ;[0 0 0] Attack
  (:Triggered
    (if (and (and (Variables|Default|GetcanAttack) (not (Variables|Default|GetIsShielded))) (== 0.0 (.z (Transformation|GetVelocity))))
      (if (not (Variables|Default|GetIsAttacking))
        (CallFunction|StopCrouching)
        (if (not (AI|Components|NavMovement|IsCrouching (Variables|Character|GetCharacterMovement)))
          (Variables|Default|SetcanAttack false)
          (Variables|Default|SetIsAttacking true)
          (Audio|PlaySound2D "/Game/Sounds/Player/SwordSwing.SwordSwing" 1.0 1.0 0.0 0 0)
          (Utilities|FlowControl|Delay 0.3)
          (bind (_outhit _returnvalue_4) (Collision|SphereTraceByChannel _returnvalue_3 _returnvalue_3 8e+01 "TraceTypeQuery1" false 0 "None"))
          (if _returnvalue_4
            (if (Actor|ActorHasTag (.HitActor (Collision|BreakHitResult _outhit)) "Enemy")
              (if (Variables|Default|GetisEmpowered)
                (Audio|PlaySound2D "/Game/Sounds/Player/EnhancedAttack.EnhancedAttack" 1.0 1.0 0.0 0 0)
                (Development|PrintString "Push Enemy")
                (Game|Damage|ApplyDamage (.HitActor (Collision|BreakHitResult _outhit)) (* _attackdamage 1.5) 0 0)
                (else
                  (Audio|PlaySound2D "/Game/Sounds/Player/Attack.Attack" 1.0 1.0 0.0 0 0)
                  (Game|Damage|ApplyDamage (.HitActor (Collision|BreakHitResult _outhit)) _attackdamage 0 0)))))
          (Utilities|FlowControl|Delay 0.3)
          (Variables|Default|SetIsAttacking false)
          (Utilities|FlowControl|Delay 0.25)
          (Variables|Default|SetcanAttack true))))))

(event Input|EnhancedActionEvents|EnhancedInputActionIA_Pause
  (params (ActionValue :type Boolean) (ElapsedSeconds :type Float%20%28double-precision%29) (TriggeredSeconds :type Float%20%28double-precision%29) (InputAction :type Input%20Action%20Object%20Reference :default "/Game/Player/Blueprints/Input/IA_Pause.IA_Pause"))
  (bind _playerinterface (Variables|Default|GetPlayerInterface))
  ;[0 0 0] Pause
  (:Triggered
    (if (Game|IsGamePaused)
      (Class|BPIPlayerInterface|PauseUnpauseGame(Message) _playerinterface false)
      (else
        (Class|BPIPlayerInterface|PauseUnpauseGame(Message) _playerinterface true)))))

(event Input|EnhancedActionEvents|EnhancedInputActionIA_Shield
  (params (ActionValue :type Float%20%28double-precision%29) (ElapsedSeconds :type Float%20%28double-precision%29) (TriggeredSeconds :type Float%20%28double-precision%29) (InputAction :type Input%20Action%20Object%20Reference :default "/Game/Player/Blueprints/Input/IA_Shield.IA_Shield"))
  (bind _walkruncrouchspeed (Variables|Default|GetWalkRunCrouchSpeed))
  (bind _charactermovement (Variables|Character|GetCharacterMovement))
  ;[0 0 0] Shield
  (:Started
    (if (and (> (Variables|Default|GetShieldHealth) 0) (and (Variables|Default|GetcanShield) (== 0.0 (.z (Transformation|GetVelocity)))))
      (CallFunction|StopCrouching)
      (if (not (AI|Components|NavMovement|IsCrouching (Variables|Character|GetCharacterMovement)))
        (Variables|/Script/Engine.CharacterMovementComponent|SetMaxWalkSpeed _charactermovement (* (.x _walkruncrouchspeed) 0.5))
        (bind _output_get (Variables|Default|SetIsShielded true))
        (Variables|Default|SetcanParry _output_get)
        (Utilities|FlowControl|Delay 0.5)
        (Variables|Default|SetcanParry false))))
  (:Canceled
    (Variables|Default|SetIsShielded false :!label _label)
    (Variables|Default|SetcanShield false)
    (Variables|/Script/Engine.CharacterMovementComponent|SetMaxWalkSpeed _charactermovement (.x _walkruncrouchspeed))
    (Utilities|FlowControl|Delay 0.25)
    (Variables|Default|SetcanShield true))
  (:Completed
    (goto _label)))

(event Game|Damage|EventAnyDamage
  (params (Damage :type Float%20%28single-precision%29) (DamageType :type Damage%20Type%20Object%20Reference) (InstigatedBy :type Controller%20Object%20Reference) (DamageCauser :type Actor%20Object%20Reference))
  (bind _returnvalue (Transformation|GetActorLocation DamageCauser))
  (bind _returnvalue_2 (Transformation|GetActorLocation))
  (bind _shieldhealth (Variables|Default|GetShieldHealth))
  ;[0 0 0] Take Damage
  (if (Variables|Default|GetCanTakeDamage)
    (if (Actor|ActorHasTag DamageCauser "Enemy")
      (if (Variables|Default|GetIsShielded)
        (if (== (Variables|Default|GetlastDirection) 1)
          (if (> (.x _returnvalue) (.x _returnvalue_2))
            (if (Variables|Default|GetcanParry) :!label _label
              (Variables|Default|SetisEmpowered true)
              (Utilities|FlowControl|Delay 1.0)
              (Variables|Default|SetisEmpowered false)
              (else
                (Character|LaunchCharacter (Math|Vector|MakeVector (Math|Conversions|ToFloat(Integer) (* (Variables|Default|GetlastDirection) (Variables|Default|GetPushSize))) 0.0 5.0) false false)
                (if (> (Variables|Default|GetShieldHealth) 0)
                  (if (== (Math|Random|RandomInteger 3) 0)
                    (Math|Integer|DecrementInt _shieldhealth
                      (:%20%20
                        (Audio|PlaySound2D "/Game/Sounds/Player/ShieldBreak.ShieldBreak" 1.0 1.0 0.0 0 0)
                        (if (== _shieldhealth 0)
                          (Class|BPIPlayerInterface|SetShieldIcon(Message) (Variables|Default|GetPlayerInterface) true))))))))
            (else
              (CallFunction|GetHit Damage :!label _label_2)))
          (elif (< (.x _returnvalue) (.x _returnvalue_2))
            (goto _label)
            (else
              (goto _label_2))))
        (else
          (goto _label_2)))
      (else
        (goto _label_2)))))

(event EventSetHealthtoMax
  (CallFunction|SetHealth (Variables|Default|GetMaxHealth)))

(event EventRepairShield
  (Variables|Default|SetShieldHealth (Variables|Default|GetMaxShieldHealth))
  (Class|BPIPlayerInterface|SetShieldIcon(Message) (Variables|Default|GetPlayerInterface) false))

(event EventTick
  (params (DeltaSeconds :type Float%20%28single-precision%29))
  (if (not (Variables|Default|GetIsShielded))
    (CallFunction|SetRotation)
    (CallFunction|UpdateMovementSound)
    (CallFunction|FallSound)
    (if (and (AI|Components|NavMovement|IsCrouching (Variables|Character|GetCharacterMovement)) (not (Variables|Default|GetCrouchpress)))
      (CallFunction|StopCrouching))))

(event EventBeginPlay
  (bind _charactermovement (Variables|Character|GetCharacterMovement))
  (bind _walkruncrouchspeed (Variables|Default|GetWalkRunCrouchSpeed))
  (CallFunction|AddMapping)
  (CallFunction|SetHealth (Variables|Default|GetMaxHealth))
  (CallFunction|InterfaceSetup)
  (Variables|/Script/Engine.CharacterMovementComponent|SetMaxWalkSpeed _charactermovement (.x _walkruncrouchspeed))
  (Variables|/Script/Engine.CharacterMovementComponent|SetMaxWalkSpeedCrouched _charactermovement (.z _walkruncrouchspeed)))

(event EventIgniteTorch
  (Rendering|SetVisibility (Variables|Default|GetTorch) true false)
  (Audio|PlaySound2D "/Game/Sounds/PickUps/Torch.Torch" 1.0 1.0 0.0 0 0))

(event EventKeyPickedUp
  (Variables|Default|SethasKey true))

(event Input|KeyboardEvents|G
  (params (Key :type Key%20Structure :default "None"))
  (:Pressed
    (Game|Damage|ApplyDamage self 1e+01 0 self)))

(fn ConstructionScript)

(fn SetHealth
  (params (Health :type Float%20%28double-precision%29))
  (bind _maxhealth (Variables|Default|GetMaxHealth))
  (bind _playerinterface (Variables|Default|GetPlayerInterface))
  (bind _output_get (Variables|Default|SetHealth (Math|Float|Clamp(Float) Health 0.0 _maxhealth)))
  (Utilities|IsValid _playerinterface
    (:Is%20Valid
      (Class|BPIPlayerInterface|SetHealthPercent(Message) _playerinterface (/ _output_get _maxhealth)))))

(fn TakeDamage
  (params (Damage :type Float%20%28double-precision%29))
  (CallFunction|SetHealth (- (Variables|Default|GetHealth) Damage))
  (if (== 0.0 (Variables|Default|GetHealth))
    (CallFunction|Die)))

(fn Die
  (bind _returnvalue (Game|GetCurrentLevelName true))
  (Game|OpenLevel(byName) (Utilities|String|StringToName _returnvalue))
  (Development|PrintString "Moriste"))

(fn CheckHasKey
  (return (Variables|Default|GethasKey)))

(fn GetAnimData
  (return (AI|Components|NavMovement|IsCrouching (Variables|Character|GetCharacterMovement)) (Variables|Default|GetIsAttacking) (.y (Variables|Default|GetWalkRunCrouchSpeed)) (Variables|Default|GetIsShielded) (not (Variables|Default|GetCanTakeDamage))))